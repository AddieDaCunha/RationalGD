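; PlayerFloatingDamage_BP is a floating damage number actor, apparently for damage involving the player.
; The PlayerDamageTextSpawned event writes the truncated damage value into its PlayerDamageText_Widget component text.
; A Fade timeline drives the text's render opacity while a Movement timeline lerps the actor straight up from its spawn location.
; The actor destroys itself when the movement finishes.
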(event `PlayerDamageTextSpawned`
  (params (DamageText :type "Float (double-precision)"))
  (bind _randomfloating (`self.RandomFloating`))
  (`|ExecutionSequence`
    (:`then_0`
      ;[1 1 1] Show Text
      (bind _asplayer_damage_text_widget (cast `/Game/Widgets/PlayerDamageText_Widget` (`WidgetComponent.GetUserWidgetObject` (`self.Widget`))))
      (bind _damage_text (`/Game/Widgets/PlayerDamageText_Widget.Damage_Text` _asplayer_damage_text_widget))
      (`TextBlock.SetText` _damage_text (`KismetTextLibrary.Conv_IntToText` (`KismetMathLibrary.FTrunc` DamageText)))
      (bind (_direction _float) (`Timeline|Fade` :!via `PlayFromStart`)
        (:`Update`
          (`Widget.SetRenderOpacity` _damage_text _float))))
    (:`then_1`
      ;[1 1 1] Movement of Text
      (set `self.RandomFloating` (`self.K2_GetActorLocation`))
      (bind (_direction_2 _movement) (`Timeline|Movement` :!via `PlayFromStart`)
        (:`Update`
          (`self.K2_SetActorLocation` (`KismetMathLibrary.VLerp` _randomfloating (+ _randomfloating (0.0 0.0 150.0)) _movement)))
        (:`Finished`
          (`self.K2_DestroyActor`))))))

(fn `UserConstructionScript`)