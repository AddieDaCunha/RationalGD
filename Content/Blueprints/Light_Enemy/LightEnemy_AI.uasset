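; AI controller for the light enemy that runs its behavior tree and relays attack requests to the controlled pawn.
; On BeginPlay it caches the pawn, stores the player character as the target and writes the initial AIState to the Blackboard.
; A looping timer named as a test repeatedly forces one fixed state into that key.
; The Pawn_Attack event calls Attack on the cached enemy.
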(event `self.ReceiveBeginPlay`
  (bind _aslight_enemy_bp (cast `/Game/Blueprints/Light_Enemy/LightEnemy_BP` (`self.K2_GetPawn`)))
  (set `self.As Light Enemy BP` _aslight_enemy_bp)
  (`self.RunBehaviorTree` "/Game/Blueprints/Light_Enemy/LightEnemyAI_BT.LightEnemyAI_BT")
  (set `self.CurrentTarget` (`GameplayStatics.GetPlayerCharacter` 0))
  (`BlackboardComponent.SetValueAsEnum` (`AIBlueprintHelperLibrary.GetBlackboard` null) "AIState" (`self.CurrentState`))
  (`KismetSystemLibrary.K2_SetTimerDelegate` (delegate `test`) 3.0 true))

(event `test`
  (bind _output_get (set `self.CurrentState` "NewEnumerator1"))
  (`BlackboardComponent.SetValueAsEnum` (`AIBlueprintHelperLibrary.GetBlackboard` null) "AIState" _output_get))

(event `Pawn_Attack`
  ;[1 1 1] Make Attack
  (`/Game/Blueprints/Light_Enemy/LightEnemy_BP.Attack` (`self.As Light Enemy BP`)))

(fn `UserConstructionScript`)