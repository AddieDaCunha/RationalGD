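; FightDirector_BP is a director for light enemy fights that triggers attacks across a list of enemies.
; On BeginPlay it binds TriggerAttack to each listed enemy's LightEnemy_AI attacking event.
; TriggerAttack calls AIAttack on every listed enemy's controller, stopping at the first failed cast.
; An unfinished grading system has its random scoring and highest-grade comparison disconnected, so it does not affect attacks.
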(event `self.ReceiveBeginPlay`
  ;[1 1 1] Enemy List
  (for _array_element (`self.EnemyList`)
    (add `/Game/Blueprints/Light_Enemy/LightEnemy_AI.Attacking` (cast `/Game/Blueprints/Light_Enemy/LightEnemy_AI` (`Pawn.GetController` _array_element) :!pure true) (delegate `Trigger Attack`))))

(event `Trigger Attack`
  ;[1 1 1] Attack function
  (for _array_element (`self.EnemyList`)
    (bind _aslight_enemy_ai (cast `/Game/Blueprints/Light_Enemy/LightEnemy_AI` (`AIBlueprintHelperLibrary.GetAIController` _array_element)))
    (`/Game/Blueprints/Light_Enemy/LightEnemy_AI.AIAttack` _aslight_enemy_ai)))

(fn `FindHighestGrade`
  (returns (Loc_HighestValue1 :type "Float (double-precision)") (Loc_HighestGradedAI1 :type "/Game/Blueprints/Light_Enemy/LightEnemy_BP Object Reference"))
  (locals (Loc_HighestValue :type "Float (double-precision)") (Loc_HighestGradedAI :type "/Game/Blueprints/Light_Enemy/LightEnemy_BP Object Reference"))
  (bind _keys (`BlueprintMapLibrary.Map_Keys` (`self.EnemyGrading`)))
  (for _array_element _keys
    (bind _output_get (set `local.Loc_HighestGradedAI` _array_element))
    (set `local.Loc_HighestGradedAI` _output_get))
  (return (`local.Loc_HighestValue`) (`local.Loc_HighestGradedAI`)))

(fn `UserConstructionScript`)