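; LightEnemy_BP is a light melee enemy that attacks and damages the player character.
; Its Attack event plays a melee montage on the mesh.
; AttackCollision overlaps with MainCharacter_BP apply fixed damage, then switch off the box's overlap events, which this graph never re-enables.
; The AI perception event is empty, and the logic to store the player and turn toward them is disconnected.
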(event `self.AIPerception.OnTargetPerceptionUpdated`
  (params (Actor :type "Actor Object Reference") (Stimulus :type "AIStimulus Structure")))

(event `self.ReceiveTick`
  (params (DeltaSeconds :type "Float (single-precision)")))

(event `Attack`
  ;[1 1 1] Attack Montage
  (`|PlayMontage` (`self.Mesh`) "/Game/Blueprints/Light_Enemy/Melee_A_Montage.Melee_A_Montage"))

(event `self.Attack Collision.OnComponentBeginOverlap`
  (params (OverlappedComponent :type "PrimitiveComponent Object Reference") (OtherActor :type "Actor Object Reference") (OtherComp :type "PrimitiveComponent Object Reference") (OtherBodyIndex :type Integer) (bFromSweep :type Boolean) (SweepResult :type "HitResult Structure (by ref)"))
  ;[1 1 1] Attack Damage
  (bind _asmain_character_bp (cast `/Game/Blueprints/MainCharacter_BP` OtherActor))
  (`GameplayStatics.ApplyDamage` _asmain_character_bp 10.0)
  (set `PrimitiveComponent.bGenerateOverlapEvents` false (`self.Attack Collision`)))

(fn `UserConstructionScript`)