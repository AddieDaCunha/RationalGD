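; Behavior Tree task for the light enemy that anchors it at its current spot and triggers an attack.
; On execute it writes the controlled pawn's location to the target location Blackboard key, then checks the Attacking flag.
; If not already attacking, it calls CallAttacking on the LightEnemy_AI controller and succeeds; otherwise it fails.
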(event `self.ReceiveExecuteAI`
  (params (OwnerController :type "AIController Object Reference") (ControlledPawn :type "Pawn Object Reference"))
  ;[1 1 1] Once reach the player then attack
  (`BTFunctionLibrary.SetBlackboardValueAsVector` (`self.BB_TargetLocation`) (`Actor.K2_GetActorLocation` ControlledPawn))
  (if (not (`BlackboardComponent.GetValueAsBool` (`AIBlueprintHelperLibrary.GetBlackboard` ControlledPawn) "Attacking"))
    (`/Game/Blueprints/Light_Enemy/LightEnemy_AI.Attacking` (cast `/Game/Blueprints/Light_Enemy/LightEnemy_AI` OwnerController :!pure true))
    (`self.FinishExecute` true)
    (else
      (`self.FinishExecute` false))))