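; BuffEnemy_BP is a melee enemy that damages the main character and rewards souls when killed.
; Attack plays a montage, while left and right collision components deal random damage on overlap, then disable their own overlap events.
; AnyDamage spawns floating damage text and reduces Health.
; At zero Health it starts the death montage and, without waiting for completion, awards souls, decrements the game mode's enemy count and destroys itself.
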(event `Attack`
  ;[1 1 1] Attack Montage
  (`|PlayMontage` (`self.Mesh`) "/Game/Blueprints/Enemies/Buff_Enemy/Attack_Special_3_Montage.Attack_Special_3_Montage"))

(event `self.Attack Collision Left.OnComponentBeginOverlap`
  (params (OverlappedComponent :type "PrimitiveComponent Object Reference") (OtherActor :type "Actor Object Reference") (OtherComp :type "PrimitiveComponent Object Reference") (OtherBodyIndex :type Integer) (bFromSweep :type Boolean) (SweepResult :type "HitResult Structure (by ref)"))
  ;[1 1 1] Attack Damage
  (bind _asmain_character_bp (cast `/Game/Blueprints/Player_Character/MainCharacter_BP` OtherActor))
  (`GameplayStatics.ApplyDamage` _asmain_character_bp (`KismetMathLibrary.RandomFloatInRange` 25.0 35.0))
  (set `PrimitiveComponent.bGenerateOverlapEvents` false (`self.Attack Collision Left`)))

(event `self.Attack Collision Right.OnComponentBeginOverlap`
  (params (OverlappedComponent :type "PrimitiveComponent Object Reference") (OtherActor :type "Actor Object Reference") (OtherComp :type "PrimitiveComponent Object Reference") (OtherBodyIndex :type Integer) (bFromSweep :type Boolean) (SweepResult :type "HitResult Structure (by ref)"))
  ;[1 1 1] Attack Damage
  (bind _asmain_character_bp (cast `/Game/Blueprints/Player_Character/MainCharacter_BP` OtherActor))
  (`GameplayStatics.ApplyDamage` _asmain_character_bp (`KismetMathLibrary.RandomFloatInRange` 25.0 35.0))
  (set `PrimitiveComponent.bGenerateOverlapEvents` false (`self.Attack Collision Right`)))

(event `self.ReceiveAnyDamage`
  (params (Damage :type "Float (single-precision)") (DamageType :type "DamageType Object Reference") (InstigatedBy :type "Controller Object Reference") (DamageCauser :type "Actor Object Reference"))
  ;[1 1 1] Show Damage Text
  (set `self.Damage` Damage)
  (bind _returnvalue (`|SpawnActorFromClass` "/Game/Blueprints/FloatingDamage_BP.FloatingDamage_BP_C" (`KismetMathLibrary.Conv_VectorToTransform` (+ (`self.K2_GetActorLocation`) (`KismetMathLibrary.MakeVector` (`KismetMathLibrary.RandomFloatInRange` -30.0 30.0) (`KismetMathLibrary.RandomFloatInRange` -30.0 30.0) (`KismetMathLibrary.RandomFloatInRange` 150.0 250.0)))) "Undefined" "OverrideRootScale" null null))
  (`/Game/Blueprints/FloatingDamage_BP.DamageTextSpawned` _returnvalue (`self.Damage`))
  ;[1 1 1] Take Damage
  (bind _output_get (set `self.Health` (- (`self.Health`) Damage)))
  (if (<= _output_get 0.0)
    (`|PlayMontage` (`self.Mesh`) "/Game/Blueprints/Enemies/Buff_Enemy/Death_Montage.Death_Montage"
      (:`then`
        ;[1 1 1] Add Currency
        (bind _asmain_character_bp (cast `/Game/Blueprints/Player_Character/MainCharacter_BP` (`GameplayStatics.GetPlayerCharacter` 0)))
        (set `/Game/Blueprints/Player_Character/MainCharacter_BP.Souls` (+ (`/Game/Blueprints/Player_Character/MainCharacter_BP.Souls` _asmain_character_bp) (`KismetMathLibrary.RandomIntegerInRange` 10 15)) _asmain_character_bp)
        ;[1 1 1] Count number of enemies
        (bind _asthird_person_game_mode (cast `/Game/Blueprints/ThirdPersonGameMode` (`GameplayStatics.GetGameMode`)))
        (set `/Game/Blueprints/ThirdPersonGameMode.NumberOfEnemies` (- (`/Game/Blueprints/ThirdPersonGameMode.NumberOfEnemies` _asthird_person_game_mode) 1) _asthird_person_game_mode)
        (`self.K2_DestroyActor`)))))

(fn `UserConstructionScript`)